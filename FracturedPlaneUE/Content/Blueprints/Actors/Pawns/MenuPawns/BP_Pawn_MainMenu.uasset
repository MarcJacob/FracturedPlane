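; Main menu pawn that shows the client main menu widget while it is the view target and removes it afterwards.
; It binds the widget's login and exit buttons, with exit quitting the game.
; Login connects to the game master server, sends an authentication request with the entered username and an empty password, and updates progress text.
; Failed connections or a disconnected authentication response report the last fail reason to the widget.
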(event Custom|OnLoginButtonClicked
  ;[1 1 1] Login & Authentication Pipeline
  (Default|OnLoggingin (Variables|Default|GetMainMenuWidget))
  (Default|SetLoggingProcessStepName (Variables|Default|GetMainMenuWidget) "Connecting...")
  (bind _returnvalue (Class|FPMasterServerConnectionSubsystem|ConnecttoGameMasterServer (Subsystems|GetFPMasterServerConnectionSubsystem)))
  (if _returnvalue
    (Class|FPMasterServerConnectionSubsystem|SendAuthenticationRequest (Subsystems|GetFPMasterServerConnectionSubsystem) (Utilities|Struct|MakeFPClientAuthenticationInfo (Utilities|String|ToString(Text) (Default|GetInputUsername (Variables|Default|GetMainMenuWidget))) ""))
    (Default|SetLoggingProcessStepName (Variables|Default|GetMainMenuWidget) "Authenticating...")
    (EventDispatchers|BindEventtoOnAuthenticationStateChanged (Subsystems|GetFPMasterServerConnectionSubsystem) (delegate Custom|OnAuthenticationResponse))
    (else
      (Default|OnLoggingFailure (Variables|Default|GetMainMenuWidget) (.lastfailreason (Variables|/Script/FracturedPlaneClientCore.FPMasterServerConnectionSubsystem|GetAuthenticationInfo (Subsystems|GetFPMasterServerConnectionSubsystem)))))))

(event Custom|OnExitGameButtonClicked
  (Game|QuitGame 0 "Quit" false))

(event Custom|OnAuthenticationResponse
  (params (State :type EAuthentificationState%20Enum :default "DISCONNECTED"))
  ;[1 1 1] Login & Authentication Pipeline
  (Utilities|FlowControl|Sequence
    (:then_0
      (EventDispatchers|UnbindEventfromOnAuthenticationStateChanged (Subsystems|GetFPMasterServerConnectionSubsystem) (delegate Custom|OnAuthenticationResponse)))
    (:then_1
      (switch Utilities|FlowControl|Switch|SwitchonEAuthentificationState State
        (:DISCONNECTED
          (Default|OnLoggingFailure (Variables|Default|GetMainMenuWidget) (.lastfailreason (Variables|/Script/FracturedPlaneClientCore.FPMasterServerConnectionSubsystem|GetAuthenticationInfo (Subsystems|GetFPMasterServerConnectionSubsystem)))))))))

(event EventOnBecomeViewTarget
  (params (PC :type Player%20Controller%20Object%20Reference))
  (CallFunction|SetupWidget))

(event EventOnEndViewTarget
  (params (PC :type Player%20Controller%20Object%20Reference))
  (Widget|RemovefromParent (Variables|Default|GetMainMenuWidget))
  (Variables|Default|SetMainMenuWidget 0))

(fn ConstructionScript)

(fn SetupWidget
  (bind _returnvalue (Game|ConstructObjectfromClass "/Game/Widgets/UI/FPWidget_ClientMainMenu.FPWidget_ClientMainMenu_C"))
  (bind _output_get (Variables|Default|SetMainMenuWidget _returnvalue))
  (UserInterface|Viewport|AddtoViewport _output_get 0)
  (Utilities|IsValid (Variables|Default|GetMainMenuWidget)
    (:Is%20Valid
      (CallFunction|RegisterMainMenuWidgetEvents))
    (:Is%20Not%20Valid
      (Development|PrintString "ERROR: Failed to Spawn Main Menu Widget !" true true "(R=1.000000,G=0.000000,B=0.000000,A=1.000000)" 2.0 "MainMenu Spawn Failure"))))

(fn RegisterMainMenuWidgetEvents
  (EventDispatchers|BindEventtoOnLoginButtonPressed (Variables|Default|GetMainMenuWidget) (EventDispatchers|CreateEvent :!event Custom|OnLoginButtonClicked))
  (EventDispatchers|BindEventtoOnExitGameButtonPressed (Variables|Default|GetMainMenuWidget) (EventDispatchers|CreateEvent :!event Custom|OnExitGameButtonClicked)))